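; Moving platform Blueprint that travels toward an end point while the player character stands inside its trigger box.
; BeginPlay caches the platform's start location and the EndPoint location, and slows the timeline's play rate.
; Overlapping the box with CharacterBp plays the timeline, lerping the platform between the two locations, and leaving the box reverses it back toward the start.
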(event `self.ReceiveBeginPlay`
  (set `self.Start_Loc` (`SceneComponent.K2_GetComponentLocation` (`self.moving_platform`)))
  (set `self.End_Loc` (`SceneComponent.K2_GetComponentLocation` (`self.end point`)))
  (`TimelineComponent.SetPlayRate` (`self.Move_Plat_Timeline`) 0.2))

(event `self.Box.OnComponentBeginOverlap`
  (params (OverlappedComponent :type "PrimitiveComponent Object Reference") (OtherActor :type "Actor Object Reference") (OtherComp :type "PrimitiveComponent Object Reference") (OtherBodyIndex :type Integer) (bFromSweep :type Boolean) (SweepResult :type "HitResult Structure (by ref)"))
  (cast `/Game/Blueprints/CharacterBp` OtherActor)
  (bind (_direction _newtrack_0) (`Timeline|Move_Plat_Timeline` :!label _label)
    (:`Update`
      (`SceneComponent.K2_SetWorldLocation` (`self.moving_platform`) (`KismetMathLibrary.VLerp` (`self.Start_Loc`) (`self.End_Loc`) _newtrack_0) false false))))

(event `self.Box.OnComponentEndOverlap`
  (params (OverlappedComponent :type "PrimitiveComponent Object Reference") (OtherActor :type "Actor Object Reference") (OtherComp :type "PrimitiveComponent Object Reference") (OtherBodyIndex :type Integer))
  (cast `/Game/Blueprints/CharacterBp` OtherActor)
  (goto _label :!via `Reverse`))

(fn `UserConstructionScript`)