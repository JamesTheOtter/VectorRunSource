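; Player character with axis movement and look, a double jump, wall running, a HUD and a hold-H tutorial widget.
; Jumps launch upward through a DoN counter that resets on landing or Walldetect overlap.
; Overlapping a RunWall-tagged actor while falling starts a timeline that, while Space is held, removes gravity, constrains height and pushes along the captured camera direction.
; Any damage, or destruction with objectives remaining, shows the death screen.
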(event `InputAxis|Rotate_Left_Right`
  (params (AxisValue :type "Float (single-precision)"))
  ;[1 1 1] Movement
  (`self.AddControllerYawInput` AxisValue))

(event `InputAxis|Forward_Backwards`
  (params (AxisValue :type "Float (single-precision)"))
  ;[1 1 1] Movement
  (`self.AddMovementInput` (`KismetMathLibrary.GetForwardVector` (`self.GetControlRotation`)) AxisValue))

(event `InputAxis|Rotate_Up_Down`
  (params (AxisValue :type "Float (single-precision)"))
  ;[1 1 1] Movement
  (`self.AddControllerPitchInput` AxisValue))

(event `self.ReceiveBeginPlay`
  (bind _returnvalue (`GameplayStatics.GetPlayerController` 0))
  (`MovementComponent.SetPlaneConstraintEnabled` (`self.CharacterMovement`) true)
  (bind _returnvalue_2 (`|CreateWidget` "/Game/HUD.HUD_C"))
  (set `self.HUD Reference` _returnvalue_2)
  (`UserWidget.AddToViewport` _returnvalue_2 0)
  (`WidgetBlueprintLibrary.SetInputMode_GameOnly` _returnvalue)
  (set `PlayerController.bShowMouseCursor` false _returnvalue))

(event `InputAxis|Left_Right`
  (params (AxisValue :type "Float (single-precision)"))
  ;[1 1 1] Movement
  (`self.AddMovementInput` (`KismetMathLibrary.GetRightVector` (`self.GetControlRotation`)) AxisValue))

(event `self.OnLanded`
  (params (Hit :type "HitResult Structure (by ref)"))
  (goto _label :!via `Reset`))

(event `InputAction|Jump`
  (params (Key :type "Key Structure"))
  (:`Pressed`
    (bind _counter (`/Engine/EditorBlueprintResources/StandardMacros.Do N` 2 :!label _label)
      (:`Exit`
        (switch `int` _counter
          (:`1`
            _)
          (:`2`
            _))
        (`self.LaunchCharacter` (0.0 0.0 300.0) false true)
        (`|PlayMontage` (`self.Mesh`) (`self.Jump Montage`)))))
  (:`Released`
    (`self.StopJumping`)))

(event `self.walldetect.OnComponentBeginOverlap`
  (params (OverlappedComponent :type "PrimitiveComponent Object Reference") (OtherActor :type "Actor Object Reference") (OtherComp :type "PrimitiveComponent Object Reference") (OtherBodyIndex :type Integer) (bFromSweep :type Boolean) (SweepResult :type "HitResult Structure (by ref)"))
  (bind _charactermovement (`self.CharacterMovement`))
  (bind _charactermovement_2 (`self.CharacterMovement`))
  (`|ExecutionSequence`
    (:`then_0`
      (goto _label :!via `Reset`))
    (:`then_1`
      (set `self.PlayerDirection` (`SceneComponent.GetForwardVector` (`self.Camera`)))
      (if (and (`self.ActorHasTag` OtherActor "RunWall") (`NavMovementComponent.IsFalling` (`self.CharacterMovement`)))
        (set `self.OnWall` true)
        (`Timeline|WallRun` :!label _label_2
          (:`Update`
            (if (> (`PlayerController.GetInputKeyTimeDown` (`GameplayStatics.GetPlayerController` 0) "SpaceBar") 0.0)
              (if (`self.OnWall`)
                (set `CharacterMovementComponent.GravityScale` 0.0 _charactermovement_2)
                (`MovementComponent.SetPlaneConstraintNormal` _charactermovement_2 (0.0 0.0 1.0))
                (`CharacterMovementComponent.AddForce` (`self.CharacterMovement`) (* (`self.PlayerDirection`) 20000.0))
                (else
                  (set `CharacterMovementComponent.GravityScale` 1.0 _charactermovement :!label _label_3)
                  (`MovementComponent.SetPlaneConstraintNormal` _charactermovement (0.0 0.0 0.0))
                  (set `self.OnWall` false)))
              (else
                (goto _label_3)))))))))

(event `self.walldetect.OnComponentEndOverlap`
  (params (OverlappedComponent :type "PrimitiveComponent Object Reference") (OtherActor :type "Actor Object Reference") (OtherComp :type "PrimitiveComponent Object Reference") (OtherBodyIndex :type Integer))
  (`|ExecutionSequence`
    (:`then_0`
      (goto _label_2 :!via `Stop`))
    (:`then_1`
      (if (`self.ActorHasTag` OtherActor "RunWall")
        (goto _label_3)))))

(event `Key|H`
  (params (Key :type "Key Structure"))
  (:`Pressed`
    (bind _returnvalue (`|CreateWidget` "/Game/TutorialWidget.TutorialWidget_C"))
    (`UserWidget.AddToViewport` _returnvalue 0))
  (:`Released`
    (`Widget.RemoveFromParent` _returnvalue)))

(event `self.ReceiveAnyDamage`
  (params (Damage :type "Float (single-precision)") (DamageType :type "DamageType Object Reference") (InstigatedBy :type "Controller Object Reference") (DamageCauser :type "Actor Object Reference"))
  (bind _returnvalue (`GameplayStatics.GetPlayerController` 0))
  (bind _returnvalue_2 (`|CreateWidget` "/Game/DeathScreen.DeathScreen_C" :!label _label_4))
  (`UserWidget.AddToViewport` _returnvalue_2 0)
  (`WidgetBlueprintLibrary.SetInputMode_UIOnlyEx` _returnvalue _returnvalue_2)
  (set `PlayerController.bShowMouseCursor` true _returnvalue)
  (`self.K2_DestroyActor`))

(event `self.ReceiveEndPlay`
  (params (EndPlayReason :type "EEndPlayReason Enum" :default "Destroyed"))
  (switch `EEndPlayReason` EndPlayReason
    (:`Destroyed`
      _)
    (:`RemovedFromWorld`
      _))
  (if (> (`KismetArrayLibrary.Array_Length` (`/Game/Objective_Component.Objectives` (`self.Objective_Component`))) 0)
    (goto _label_4)))

(fn `UserConstructionScript`)