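; Objective_A is a trigger-volume objective that the player completes by entering its box, which the construction script sizes from the Size variable.
; Shortly after BeginPlay it registers ObjectiveName with the player character's ObjectiveComponent and stores the returned reference.
; When a CharacterBp overlaps the box, it sets that objective's status to true, removes it from the Objectives array, reassigns the array and destroys itself.
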(event `self.ReceiveBeginPlay`
  (`KismetSystemLibrary.Delay` 0.5)
  (bind _object_created (`/Game/Objective_Component.Add Objective` (`/Game/Blueprints/CharacterBp.Objective_Component` (cast `/Game/Blueprints/CharacterBp` (`GameplayStatics.GetPlayerCharacter` 0) :!pure true)) (`self.Objective Name`)))
  (set `self.Objective Reference` _object_created))

(event `self.Box.OnComponentBeginOverlap`
  (params (OverlappedComponent :type "PrimitiveComponent Object Reference") (OtherActor :type "Actor Object Reference") (OtherComp :type "PrimitiveComponent Object Reference") (OtherBodyIndex :type Integer) (bFromSweep :type Boolean) (SweepResult :type "HitResult Structure (by ref)"))
  (bind _objective_reference (`self.Objective Reference`))
  (bind _objective_component (`/Game/Blueprints/CharacterBp.Objective_Component` (cast `/Game/Blueprints/CharacterBp` (`GameplayStatics.GetPlayerCharacter` 0) :!pure true)))
  (bind _objectives (`/Game/Objective_Component.Objectives` _objective_component))
  (cast `/Game/Blueprints/CharacterBp` OtherActor)
  (`/Game/Objective_Component.Set Objective Status` (`/Game/Blueprints/CharacterBp.Objective_Component` (cast `/Game/Blueprints/CharacterBp` (`GameplayStatics.GetPlayerCharacter` 0) :!pure true)) _objective_reference true)
  (`KismetArrayLibrary.Array_RemoveItem` _objectives _objective_reference)
  (set `/Game/Objective_Component.Objectives` _objectives _objective_component)
  (`self.K2_DestroyActor`))

(fn `UserConstructionScript`
  (`BoxComponent.SetBoxExtent` (`self.Box`) (`self.Size`) true))