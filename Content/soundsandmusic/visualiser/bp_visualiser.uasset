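; Audio visualiser actor that plays its Audio from the start on BeginPlay and can build a grid of cube actors.
; SpawnGrid spawns Bp_cube actors at spaced offsets from the actor's location, wrapping at the square root of the cube count, and stores them in BpArray.
; Nothing in these graphs calls SpawnGrid or drives the cubes from the audio.
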(event `self.ReceiveBeginPlay`
  (`AudioComponent.Play` (`self.Audio`) 0.0))

(fn `SpawnGrid`
  (locals (NewLocalVar_0 :type "Object Object Reference"))
  (bind _distance (`self.distance`))
  (for _ (range (`self.NumberOfCubes`))
    (bind _returnvalue (`|SpawnActorFromClass` "/Game/soundsandmusic/visualiser/bp_cube.bp_cube_C" (`KismetMathLibrary.MakeTransform` (+ (`KismetMathLibrary.MakeVector` (* (`self.Row`) _distance) (* (`self.column`) _distance)) (`self.K2_GetActorLocation`))) "AlwaysSpawn" "OverrideRootScale" null null))
    (`KismetArrayLibrary.Array_Add` (`self.bp_array`) _returnvalue)
    (`/Engine/EditorBlueprintResources/StandardMacros.IncrementInt` (`self.Row`)
      (:`  `
        (if (== (`self.Row`) (`KismetMathLibrary.FTrunc` (`KismetMathLibrary.Sqrt` (`KismetMathLibrary.Conv_IntToDouble` (`self.NumberOfCubes`)))))
          (`/Engine/EditorBlueprintResources/StandardMacros.IncrementInt` (`self.column`)
            (:`  `
              (set `self.Row` 0))))))))

(fn `UserConstructionScript`)